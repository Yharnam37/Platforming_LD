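; BP_Turret is a turret that turns toward and shoots at a BPA_Platforming character inside its detection sphere.
; Sphere overlap stores the character and starts two looping timers for shooting and targeting, which an IsInRange flag gates rather than clearing on exit.
; Targeting eases the actor's yaw toward the character with RInterpTo, and shooting plays a sound and spawns BP_Bullet at the Arrow's transform.
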(event OnComponentBeginOverlap(Sphere)
  (params (OverlappedComponent :type Primitive%20Component%20Object%20Reference) (OtherActor :type Actor%20Object%20Reference) (OtherComp :type Primitive%20Component%20Object%20Reference) (OtherBodyIndex :type Integer) (bFromSweep :type Boolean) (SweepResult :type Hit%20Result%20Structure%20%28by%20ref%29))
  (bind _asbpa_platforming (Utilities|Casting|CastToBPA_Platforming OtherActor))
  ;[0.15 0.15 0.15 0.5] tire
  (Utilities|Time|SetTimerbyEvent (delegate Custom|Shoot) (Variables|Default|GetShoot%20per%20sec) true true)
  (Variables|Default|SetAs%20BPA%20Platforming%20Character _asbpa_platforming)
  (Variables|Default|SetIs%20in%20range true)
  ;[0.15 0.15 0.15 0.5] Ciblage
  (Utilities|Time|SetTimerbyEvent (delegate Custom|Target) (Variables|Default|GetSpeed%20lock%20target) true true))

(event OnComponentEndOverlap(Sphere)
  (params (OverlappedComponent :type Primitive%20Component%20Object%20Reference) (OtherActor :type Actor%20Object%20Reference) (OtherComp :type Primitive%20Component%20Object%20Reference) (OtherBodyIndex :type Integer))
  (Utilities|Casting|CastToBPA_Platforming OtherActor)
  (Variables|Default|SetIs%20in%20range false))

(event Custom|Shoot
  ;[0.15 0.15 0.15 0.5] tire
  (if (Variables|Default|GetIs%20in%20range)
    (Audio|PlaySoundatLocation "/Game/Sound/Shoot.Shoot" (Transformation|GetWorldLocation (Variables|Default|GetCylinder)) "0, 0, 0" 1.0 1.0 0.0 0 0 0 0)
    (Game|SpawnActorfromClass "/Game/Blueprints/BP_Bullet.BP_Bullet_C" (Transformation|GetWorldTransform (Variables|Default|GetArrow)) "Undefined" "MultiplyWithRoot" 0 0)))

(event Custom|Target
  (bind _as_bpa_platforming_character (Variables|Default|GetAs%20BPA%20Platforming%20Character))
  ;[0.15 0.15 0.15 0.5] Ciblage
  (Utilities|IsValid _as_bpa_platforming_character
    (:Is%20Valid
      (if (Variables|Default|GetIs%20in%20range)
        (Transformation|SetActorRotation (Math|Rotator|MakeRotator 0.0 0.0 (.yaw (Math|Interpolation|RInterpTo (Transformation|GetWorldRotation (Variables|Default|GetDefaultSceneRoot)) (Math|Rotator|MakeRotator 0.0 0.0 (.yaw (Math|Rotator|FindLookatRotation (Transformation|GetActorLocation) (Transformation|GetActorLocation _as_bpa_platforming_character)))) (Utilities|Time|GetWorldDeltaSeconds) (Variables|Default|GetSpeed%20roation)))))))))

(event EventBeginPlay)

(fn ConstructionScript)